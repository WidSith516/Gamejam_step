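; Dialogue component that plays DataTable-driven conversations through a WBP_Dialogue widget.
; Each row supplies text, sound, portrait values, key and help flags, an end marker, and optional branching into options that jump to other rows.
; Widget events for finished writing and option selection advance the flow, while swapping Enhanced Input mapping contexts gates skip, next paragraph and close.
; Closing restores default input and signals the finished NPC talk.
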(event Custom|StartDialogue
  (params (Data%20Table%20in :type Data%20Table%20Object%20Reference%20%28by%20ref%29))
  ;[1 1 1] 注释
  (Variables|Default|SetData%20Table%20In Data%20Table%20in)
  (UserInterface|Viewport|AddtoViewport (Variables|Default|GetUI%20Dialogue) 0)
  (CallFunction|GetDataTableRows)
  (CallFunction|UIDisplay))

(event Custom|isDialogueFinishied
  ;[1 1 1] Common
  (CallFunction|DisableMappingContext "/Game/Input/IMC_SkipDialogue.IMC_SkipDialogue")
  (CallFunction|CheckNextDialogue))

(event Custom|ReadDataTable
  ;[1 1 1] 读取数据库
  ;;[1 1 1] 获得row数据
  (bind _returnvalue (Utilities|GetDataTableRow (Variables|Default|GetData%20Table%20In) (Utilities|Array|Get(acopy) (Variables|Default|GetOut%20Row%20Names) (Variables|Default|GetCurrentRow)))
    (:then
      (Variables|Default|SetSE%201 (.CPV_1 (Utilities|Struct|BreakS_DialogueSystemLast _returnvalue)))
      (Variables|Default|SetSE%202 (.CPV_2 (Utilities|Struct|BreakS_DialogueSystemLast _returnvalue)))
      (Variables|Default|SetCPV (.SE (Utilities|Struct|BreakS_DialogueSystemLast _returnvalue)))
      (CallFunction|GetWitchKey (.GetKey2 (Utilities|Struct|BreakS_DialogueSystemLast _returnvalue)) (.GetKey3 (Utilities|Struct|BreakS_DialogueSystemLast _returnvalue)) (.GetKey4 (Utilities|Struct|BreakS_DialogueSystemLast _returnvalue)))
      (Variables|Default|SetGet%20Help (.GetHelp (Utilities|Struct|BreakS_DialogueSystemLast _returnvalue)))
      (CallFunction|CurrentGetHelp)
      (Variables|Default|SetIsLast? (.Last (Utilities|Struct|BreakS_DialogueSystemLast _returnvalue))) ; 获取每个row的last标志
      (bind _output_get (Variables|Default|SetBranchin (.branchin (Utilities|Struct|BreakS_DialogueSystemLast _returnvalue))))
      (if _output_get
        (Default|AddOption (Variables|Default|GetUI%20Dialogue) (.NextDialogueID (Utilities|Struct|BreakS_DialogueSystemLast _returnvalue)))
        (else
          (Default|StartWriting (Variables|Default|GetUI%20Dialogue) (Utilities|String|ToString(Text) (.DialogueText (Utilities|Struct|BreakS_DialogueSystemLast _returnvalue))) (Variables|Default|GetSE%201) (Variables|Default|GetSE%202))
          (Audio|PlaySound2D (Variables|Default|GetCPV) 1.0 1.0 0.0 0 0))))))

(event Custom|GetDataTableRows
  ;[1 1 1] 注释
  (bind _outrownames (DataTable|GetDataTableRowNames (Variables|Default|GetData%20Table%20In)))
  (Variables|Default|SetOut%20Row%20Names _outrownames))

(event Custom|UIDisplay
  ;[1 1 1] Common
  (EventDispatchers|BindEventtoUpdateDialogueText (Variables|Default|GetUI%20Dialogue) (delegate Custom|jump%20to%20option%20dialogue))
  (CallFunction|ReadDataTable)
  (CallFunction|EnableMappingContext "/Game/Input/IMC_SkipDialogue.IMC_SkipDialogue")
  (EventDispatchers|BindEventtoFinishWriting (Variables|Default|GetUI%20Dialogue) (delegate Custom|isDialogueFinishied))
  (CallFunction|DisableMappingContext "/Game/FirstPerson/Input/IMC_Default.IMC_Default")
  (CallFunction|DisableMappingContext "/Game/Input/IMC_CloseDialogue.IMC_CloseDialogue"))

(event Custom|CheckNextDialogue
  ;[1 1 1] 检测下一行
  (Math|Integer|IncrementInt (Variables|Default|GetCurrentRow)
    (:%20%20
      (if (Variables|Default|GetIsLast?) ; false能翻页，true能关闭对话。
        (CallFunction|DisableMappingContext "/Game/Input/IMC_NextParagraph.IMC_NextParagraph")
        (CallFunction|EnableMappingContext "/Game/Input/IMC_CloseDialogue.IMC_CloseDialogue")
        (Variables|Default|SetCurrentRow 0)
        (else
          (CallFunction|DisableMappingContext "/Game/Input/IMC_CloseDialogue.IMC_CloseDialogue")
          (CallFunction|EnableMappingContext "/Game/Input/IMC_NextParagraph.IMC_NextParagraph"))))))

(event Custom|设置当前回复索引
  (params (IndexNow :type Integer))
  (Variables|Default|SetNextDialogueIndex IndexNow))

(event Custom|CurrentOption
  (params (NextDialogueID :type Map%20of%20Strings%20to%20Integers))
  ;[0.2552 0.2552 0.2552] 通过IsOption判断有多少的选项。
)

(event Custom|jump%20to%20option%20dialogue
  ;[1 1 1] Common
  (bind _output_get (Variables|Default|SetCurrentRow (Variables|/Game/UI/UMG/WBP_Dialogue.WBP_Dialogue_C|Getoption%20Dialogue%20ID (Variables|Default|GetUI%20Dialogue))))
  (if (== _output_get 0)
    (CallFunction|DisableMappingContext "/Game/Input/IMC_NextParagraph.IMC_NextParagraph")
    (CallFunction|DisableMappingContext "/Game/Input/IMC_SkipDialogue.IMC_SkipDialogue")
    (CallFunction|EnableMappingContext "/Game/Input/IMC_CloseDialogue.IMC_CloseDialogue")
    (else
      (bind _nextdialoguetext (CallFunction|GetCurrentDialogue (- _output_get 1)))
      (Default|StartWriting (Variables|Default|GetUI%20Dialogue) (Utilities|String|ToString(Text) _nextdialoguetext)))))

(event Input|EnhancedActionEvents|EnhancedInputActionIA_SkipDialogue
  (params (ActionValue :type Boolean) (ElapsedSeconds :type Float%20%28double-precision%29) (TriggeredSeconds :type Float%20%28double-precision%29) (InputAction :type Input%20Action%20Object%20Reference :default "/Game/Input/Actions/IA_SkipDialogue.IA_SkipDialogue"))
  ;[1 0.4156 0.4156] 跳过对话
  (Default|SkipWriting (Variables|Default|GetUI%20Dialogue)))

(event Input|EnhancedActionEvents|EnhancedInputActionIA_CloseDialogue
  (params (ActionValue :type Boolean) (ElapsedSeconds :type Float%20%28double-precision%29) (TriggeredSeconds :type Float%20%28double-precision%29) (InputAction :type Input%20Action%20Object%20Reference :default "/Game/Input/Actions/IA_CloseDialogue.IA_CloseDialogue"))
  ;[1 0.4156 0.4156] 结束对话
  (Widget|RemovefromParent (Variables|Default|GetUI%20Dialogue))
  (CallFunction|EnableMappingContext "/Game/FirstPerson/Input/IMC_Default.IMC_Default")
  (Default|CallFinishedTalkwithNpc) ; 记录下结束对话的npc名字，然后存下来，如果射线检测到存下来的名字，就不触发互动
)

(event Input|EnhancedActionEvents|EnhancedInputActionIA_NextParagraph
  (params (ActionValue :type Boolean) (ElapsedSeconds :type Float%20%28double-precision%29) (TriggeredSeconds :type Float%20%28double-precision%29) (InputAction :type Input%20Action%20Object%20Reference :default "/Game/Input/Actions/IA_NextParagraph.IA_NextParagraph"))
  ;[1 0.4156 0.4156] 跳过文本
  (CallFunction|ReadDataTable)
  (CallFunction|DisableMappingContext "/Game/Input/IMC_NextParagraph.IMC_NextParagraph")
  (CallFunction|EnableMappingContext "/Game/Input/IMC_SkipDialogue.IMC_SkipDialogue"))

(event EventBeginPlay
  ;[1 1 1] Begin play
  (bind _returnvalue (UserInterface|CreateWidget "/Game/UI/UMG/WBP_Dialogue.WBP_Dialogue_C"))
  (Variables|Default|SetUI%20Dialogue _returnvalue))

(event EventTick
  (params (DeltaSeconds :type Float%20%28single-precision%29)))

(fn GetCurrentDialogue
  (params (NextDialogueID :type Integer))
  (bind _returnvalue (Utilities|GetDataTableRow (Variables|Default|GetData%20Table%20In) (Utilities|Array|Get(acopy) (Variables|Default|GetOut%20Row%20Names) NextDialogueID))
    (:then
      (bind _output_get (LocalVariables|SetNewLocalVar (.DialogueText (Utilities|Struct|BreakS_DialogueSystemLast _returnvalue))))
      (return _output_get))))

(fn GetOptions
  (params (NextDialogueID :type Map%20of%20Strings%20to%20Integers))
  ;[1 1 1] 能够载入，但是需要手动切换对话才能够读取row的数据
)

(fn GetIndex
  (params (NextDialogueIndex :type Integer))
  (Variables|Default|SetNextDialogueIndex NextDialogueIndex))

(fn CurrentGetHelp
  (bind _output_get (Variables|Default|SetHelp_GetNum (stale _output_get_2)))
  (if (Variables|Default|GetGet%20Help)
    (bind _output_get_2 (Variables|Default|SetHelp_GetNum (+ _output_get 1)))))

(fn CurrentGetKey
  (bind _output_get (Variables|Default|SetKey_GetNum (stale _output_get_2)))
  (if (Variables|Default|GetGet%20Key)
    (bind _output_get_2 (Variables|Default|SetKey_GetNum (+ _output_get 1)))))

(fn GetWitchKey
  (params (key2 :type Integer) (key3 :type Integer) (key4 :type Integer))
  (Utilities|FlowControl|Sequence
    (:then_0
      (if (== key2 1)
        (Variables|Default|SetGetKey2 true)
        (Development|PrintString "key2")))
    (:then_1
      (if (== key3 1)
        (Variables|Default|SetGetKey3 true)
        (Development|PrintString "key3")))
    (:then_2
      (if (== key4 1)
        (Variables|Default|SetGetKey4 true)
        (Development|PrintString "key4")))))