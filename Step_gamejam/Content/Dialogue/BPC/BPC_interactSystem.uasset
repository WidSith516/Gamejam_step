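; Player component on BP_FirstPersonCharacter that detects NPCs ahead and starts their dialogue.
; Each tick a short forward object trace from the capsule looks for actors with BPC_NPCInfo.
; Target changes toggle the WBP_interaction prompt and IMC_interact mapping context, so the interact input is enabled only while an NPC is targeted.
; Interacting hides the prompt, disables that context and passes the NPC's DataTable to BPC_DialogueSystem.
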(event Custom|Update%20InteractInfo
  (bind _as_bp_first_person_character (Variables|Default|GetAs%20BP%20First%20Person%20Character))
  (bind _capsulecomponent (Variables|/Script/Engine.Character|GetCapsuleComponent _as_bp_first_person_character))
  (bind _returnvalue (Transformation|GetWorldLocation _capsulecomponent))
  (bind _returnvalue_2 (+ _returnvalue "0.000000,0.000000,50.000000"))
  ;[1 1 1] 射线检测显示互动ui
  (bind (_outhit _returnvalue_3) (Collision|LineTraceForObjects _returnvalue_2 (+ _returnvalue_2 (* (Math|Vector|GetForwardVector _capsulecomponent) 300)) (Variables|Default|GetObject%20Types) false 0 "None"))
  (if _returnvalue_3
    (bind _output_get (Variables|Default|SetOut%20Hit _outhit))
    (if (not (== (.hitactor _output_get) (Variables|Default|GetHit%20Actor)))
      (Utilities|IsValid (Actor|GetComponentbyClass (.hitactor _output_get) "/Game/Dialogue/BPC/BPC_NPCInfo.BPC_NPCInfo_C")
        (:Is%20Valid
          (CallFunction|ShowTarget)
          (Variables|Default|SetHit%20Actor (.hitactor _output_get)))
        (:Is%20Not%20Valid
          (CallFunction|ClearTarget))))
    (else
      (CallFunction|ClearTarget))))

(event Custom|ClearTarget
  ;[1 1 1] 优化，未检测到物体不用一直触发 no show
  (if (Variables|Default|GetHasTarget)
    (CallFunction|UpdateInteractWidget false)
    (Variables|Default|SetHasTarget false)
    (CallFunction|DisableMappingContext "/Game/Input/IMC_interact.IMC_interact")
    (Variables|Default|SetHit%20Actor 0)))

(event Custom|ShowTarget
  ;[1 1 1] 显示交互键
  (CallFunction|UpdateInteractWidget true)
  (Variables|Default|SetHasTarget true)
  (CallFunction|EnableMappingContext "/Game/Input/IMC_interact.IMC_interact"))

(event Custom|Start%20talk
  ;[1 1 1] 进入对话系统
  (CallFunction|DisableMappingContext "/Game/Input/IMC_interact.IMC_interact")
  (bind _datatable (Variables|/Game/Dialogue/BPC/BPC_NPCInfo.BPC_NPCInfo_C|GetDataTable (Actor|GetComponentbyClass (Variables|Default|GetHit%20Actor) "/Game/Dialogue/BPC/BPC_NPCInfo.BPC_NPCInfo_C"))
    (:then
      (Default|StartDialogue (Actor|GetComponentbyClass (Variables|Default|GetAs%20BP%20First%20Person%20Character) "/Game/Dialogue/BPC/BPC_DialogueSystem.BPC_DialogueSystem_C") _datatable))
    (:else)))

(event Input|EnhancedActionEvents|EnhancedInputActionIA_Interact
  (params (ActionValue :type Boolean) (ElapsedSeconds :type Float%20%28double-precision%29) (TriggeredSeconds :type Float%20%28double-precision%29) (InputAction :type Input%20Action%20Object%20Reference :default "/Game/Input/Actions/IA_Interact.IA_Interact"))
  ;[1 1 1] 使用交互
  (CallFunction|UpdateInteractWidget false)
  (CallFunction|StartTalk))

(event EventBeginPlay
  ;[1 1 1] 注释
  (bind _asbp_first_person_character (Utilities|Casting|CastToBP_FirstPersonCharacter (Components|GetOwner)))
  (Variables|Default|SetAs%20BP%20First%20Person%20Character _asbp_first_person_character)
  (bind _returnvalue (UserInterface|CreateWidget "/Game/UI/UMG/WBP_interaction.WBP_interaction_C"))
  (bind _output_get (Variables|Default|Setinteract%20widget _returnvalue))
  (UserInterface|Viewport|AddtoViewport _output_get 0)
  (CallFunction|UpdateInteractWidget false))

(event EventTick
  (params (DeltaSeconds :type Float%20%28single-precision%29))
  ;[1 1 1] 射线检测显示互动ui
  (CallFunction|UpdateInteractInfo))

(fn UpdateInteractWidget
  (params (show :type Boolean))
  (bind _interact_widget (Variables|Default|Getinteract%20widget))
  (if show
    (Widget|SetVisibility _interact_widget "Visible")
    (else
      (Widget|SetVisibility _interact_widget "Hidden"))))