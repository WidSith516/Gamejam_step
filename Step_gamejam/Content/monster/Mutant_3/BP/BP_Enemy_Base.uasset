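; Base enemy character for Mutant_3 that chases the player, attacks up close and lunges when near.
; BeginPlay starts a repeating AIMoveTo chase that tries a montage attack at very short range after each move.
; Tick launches it horizontally toward the player with a jump montage, but IsJumping is only self-assigned, never set true.
; AI perception sets the blackboard ChaseTarget and AttentionStamina for actors tagged as running-footstep or ring sounds.
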(event OnPerceptionUpdated(AIPerception)
  (params (UpdatedActors :type Array%20of%20Actor%20Object%20References))
  (for _array_element UpdatedActors
    (Class|AIPerceptionComponent|GetActorsPerception (Variables|Default|GetAIPerception) _array_element)
    (if (or (Actor|ActorHasTag _array_element "Soundtype_footstep_Run") (Actor|ActorHasTag _array_element "Soundtype_Ring"))
      (AI|Components|Blackboard|SetValueasObject (AI|GetBlackboard 0) (Variables|Default|GetChaseTarget) _array_element)
      (Variables|Default|SetAttentionStamina 1e+01))))

(event Custom|Chase%20player
  (AI|AIMoveTo self "0, 0, 0" (Game|GetPlayerCharacter 0) 5.0 false
    (:OnSuccess
      (Utilities|FlowControl|Delay 2.0))
    (:OnFail
      _))
  (CallFunction|ChasePlayer)
  (CallFunction|AttackPlayer))

(event Custom|Attack%20player
  (if (< (Transformation|GetDistanceTo (Variables|Default|GetPlayerRef)) 1e+01)
    (Animation|Montage|PlayMontage (Variables|Character|GetMesh) "/Game/monster/Mutant_3/Demo/Anim_Creature_Sit_Attack_7_Montage.Anim_Creature_Sit_Attack_7_Montage")))

(event EventOnLanded
  (params (Hit :type Hit%20Result%20Structure%20%28by%20ref%29))
  (Variables|Default|SetIs%20Jumping false))

(event EventTick
  (params (DeltaSeconds :type Float%20%28single-precision%29))
  (Utilities|Time|SetTimerbyEvent 0 DeltaSeconds :!label _label)
  (if (<= (Transformation|GetDistanceTo (stale _output_get)) 2e+02)
    (if (not (Variables|Default|GetIs%20Jumping))
      (bind _output_get (Variables|Default|SetPlayerRef (Game|GetPlayerCharacter 0)))
      (Variables|Default|SetIs%20Jumping (Variables|Default|GetIs%20Jumping))
      (Character|LaunchCharacter (Math|Vector|MakeVector (.x (* (Math|Vector|Normalize (- (Transformation|GetActorLocation _output_get) (Transformation|GetActorLocation self)) 0.01) "10.000000,10.000000,0.000000")) (.y (* (Math|Vector|Normalize (- (Transformation|GetActorLocation _output_get) (Transformation|GetActorLocation self)) 0.01) "10.000000,10.000000,0.000000")) 0.0) true true)
      (Animation|PlayAnimMontage "/Game/monster/Mutant_3/Demo/JumpInToVent_CC3+_Caleb_TempMotion1_Montage.JumpInToVent_CC3+_Caleb_TempMotion1_Montage" 1.0 "None")
      (Utilities|FlowControl|Delay 2.0)
      (goto _label))))

(event EventBeginPlay
  (CallFunction|ChasePlayer)
  (Animation|Montage|PlayMontage (Variables|Character|GetMesh) "/Game/monster/Mutant_3/Demo/MG_InfernoAttack_Montage.MG_InfernoAttack_Montage"))

(fn ConstructionScript)