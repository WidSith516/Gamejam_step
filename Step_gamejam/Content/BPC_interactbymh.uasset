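; BPC_interactbymh is an interaction Blueprint, named as a component, that lets the player trigger objects they look at.
; On the interact input press, it casts the player pawn to BP_FirstPersonCharacter and line-traces 800 units forward from the first-person camera on TraceTypeQuery3.
; A hit actor implementing BI_interact receives EventInteractMessage.
; The trace leaves persistent debug lines drawn in the world.
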(event Input|ActionEvents|InputActioninteract
  (params (Key :type Key%20Structure :default "None"))
  (:Pressed
    (bind _asbp_first_person_character (Utilities|Casting|CastToBP_FirstPersonCharacter (Game|Player|GetPlayerPawn 0)))
    (bind (_outhit _returnvalue) (Collision|LineTraceByChannel (Transformation|GetWorldLocation (Variables|/Game/FirstPerson/Blueprints/BP_FirstPersonCharacter.BP_FirstPersonCharacter_C|GetFirstPersonCamera _asbp_first_person_character)) (+ (Transformation|GetWorldLocation (Variables|/Game/FirstPerson/Blueprints/BP_FirstPersonCharacter.BP_FirstPersonCharacter_C|GetFirstPersonCamera _asbp_first_person_character)) (* (Math|Vector|GetForwardVector (Variables|/Game/FirstPerson/Blueprints/BP_FirstPersonCharacter.BP_FirstPersonCharacter_C|GetFirstPersonCamera _asbp_first_person_character)) 800)) "TraceTypeQuery3" false 0 "Persistent"))
    (if _returnvalue
      (if (Utilities|DoesObjectImplementInterface (.HitActor (Collision|BreakHitResult _outhit)) "/Game/FirstPerson/Blueprints/BI_interact.BI_interact_C")
        (Class|BIInteract|EventInteract(Message) (.HitActor (Collision|BreakHitResult _outhit)))))))