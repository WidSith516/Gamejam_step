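; Final door interactable that resolves the game's ending from flags on NewGameInstance.
; Interacting runs a collapsed check that references five key flags, then CeremonyPlatform picks ending A or B, both meant to destroy all BP_Enemy_Base actors.
; Ending B then steps the game instance's Textindex through timed lines and quits.
; A second text-and-quit sequence and a short Textindex message exist but are disconnected, so ending A only attempts the enemy cleanup.
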(event Custom|finaldoor
  (bind _asnew_game_instance (Utilities|Casting|CastToNewGameInstance (Game|GetGameInstance)))
  (if (|CollapseGraph _asnew_game_instance _asnew_game_instance _asnew_game_instance _asnew_game_instance _asnew_game_instance)
    (if (Variables|/Game/SE/NewGameInstance.NewGameInstance_C|GetCeremony%20Platform _asnew_game_instance)
      (bind _asbp_enemy_base (Utilities|Casting|CastToBP_Enemy_BaseClass "/Game/monster/Mutant_3/BP/BP_Enemy_Base.BP_Enemy_Base_C"))
      (bind _outactors (Actor|GetAllActorsOfClass _asbp_enemy_base))
      ;[1 1 1] 结局A
      (Actor|DestroyActor _outactors)
      (else
        (bind _asbp_enemy_base_2 (Utilities|Casting|CastToBP_Enemy_BaseClass "/Game/monster/Mutant_3/BP/BP_Enemy_Base.BP_Enemy_Base_C"))
        ;[1 1 1] 结局B
        (bind _outactors_2 (Actor|GetAllActorsOfClass _asbp_enemy_base_2))
        (Actor|DestroyActor _outactors_2)
        (|CollapseGraph_1)))))

(event EventEventInteract
  (CallFunction|Finaldoor))

(fn ConstructionScript)