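; Locked door Blueprint that responds to interaction with audio and an on-screen sign instead of opening.
; EventInteract is gated by a DoOnce, reset after a short retriggerable delay, and calls Opendoor to play the Opda sound and changetextindex to show feedback.
; changetextindex sets the shared Textindex on NewGameInstance, adds a new Signs_bp widget to the viewport, then clears the index after a delay.
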(event Custom|Open%20door
  (Audio|Components|Audio|Play (Variables|Default|Getopda) 0.0))

(event Custom|change%20text%20index
  (bind _asnew_game_instance (Utilities|Casting|CastToNewGameInstance (Game|GetGameInstance)))
  (Variables|/Game/SE/NewGameInstance.NewGameInstance_C|Settextindex _asnew_game_instance 6)
  (bind _returnvalue (UserInterface|CreateWidget "/Game/SE/signs/signs_bp.signs_bp_C" (Game|GetPlayerController 0)))
  (UserInterface|Viewport|AddtoViewport _returnvalue 0)
  (Utilities|FlowControl|Delay 3.0)
  (Variables|/Game/SE/NewGameInstance.NewGameInstance_C|Settextindex _asnew_game_instance 0))

(event EventEventInteract
  ;[1 1 1] logic
  (Utilities|FlowControl|DoOnce false :!label _label
    (:Completed
      (CallFunction|OpenDoor)
      (CallFunction|ChangeTextIndex)
      (Utilities|FlowControl|RetriggerableDelay 1.1)
      (goto _label Reset))))

(fn ConstructionScript)