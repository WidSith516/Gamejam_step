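; Interactable door Blueprint that swings open on interaction and closes when an overlap with its Box ends.
; Timelines drive rotator lerps on the Door component, from its current rotation to a 90-degree turn and from that turn back to zero, each alongside what appears to be a sound.
; A DoOnce reset after a short retriggerable delay throttles repeated interaction.
; Closing runs on every end overlap, without checking whether the door is open.
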(event OnComponentEndOverlap(Box)
  (params (OverlappedComponent :type Primitive%20Component%20Object%20Reference) (OtherActor :type Actor%20Object%20Reference) (OtherComp :type Primitive%20Component%20Object%20Reference) (OtherBodyIndex :type Integer))
  ;[1 1 1] close door
  (Audio|Components|Audio|Play (Variables|Default|Getclda) 0.0)
  (bind _door_track (Timeline|时间轴 PlayFromStart)
    (:Update
      (Transformation|SetRelativeRotation (Variables|Default|Getdoor) (Math|Rotator|Lerp(Rotator) "0.000000,90.000000,0.000000" "0, 0, 0" _door_track true) false false))))

(event Custom|Open%20door
  (bind _door (Variables|Default|Getdoor))
  ;[1 1 1] open door-interaction
  (Audio|Components|Audio|Play (Variables|Default|Getopda) 0.0)
  (bind _door_track (Timeline|opendoor PlayFromStart)
    (:Update
      (Transformation|SetRelativeRotation _door (Math|Rotator|Lerp(Rotator) (Variables|/Script/Engine.SceneComponent|GetRelativeRotation _door) "0.000000,90.000000,0.000000" _door_track true) false false))))

(event EventEventInteract
  ;[1 1 1] logic
  (Utilities|FlowControl|DoOnce false :!label _label
    (:Completed
      (CallFunction|OpenDoor)
      (Utilities|FlowControl|RetriggerableDelay 1.1)
      (goto _label Reset))))

(fn ConstructionScript)