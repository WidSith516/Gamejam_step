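; Landline phone Blueprint that plays ring, pickup or hangup sounds.
; On BeginPlay it checks the Isplayingsound flag and stops all three audio components if it is set.
; Otherwise it switches on State and plays the matching Ring, Pickup or Hangup sound from the start.
; The construction script is empty.
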(event EventBeginPlay
  (if (Variables|Default|Getisplayingsound)
    (Audio|Components|Audio|Stop (Variables|Default|Getring))
    (else
      (switch Utilities|FlowControl|Switch|Switchonlandline (Variables|Default|Getstate)
        (:NewEnumerator0
          (Audio|Components|Audio|Play (Variables|Default|Getring) 0.0))
        (:NewEnumerator1
          (Audio|Components|Audio|Play (Variables|Default|Getpickup) 0.0))
        (:NewEnumerator2
          (Audio|Components|Audio|Play (Variables|Default|Gethangup) 0.0))))))

(fn ConstructionScript)