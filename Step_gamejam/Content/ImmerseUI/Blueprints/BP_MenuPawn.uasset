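; BP_MenuPawn is the player pawn for menus, serving as the camera that moves between menu screens.
; On BeginPlay it adds the menu input mapping, shows the cursor and caches BP_WidgetWorker.
; OpenScreen closes the previous screen, teleports to the new screen's CineCamera, copies its post-process and focus settings, then opens it.
; Enhanced Input actions forward exit and control presses through calls, and a debug key opens the loading screen.
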(event Custom|OpenScreen
  (params (Screen :type BP%20Screen%20BG%20Object%20Reference))
  (bind _cinecamera (Variables|/Game/ImmerseUI/Blueprints/Screens/BP_ScreenBG.BP_ScreenBG_C|GetCineCamera Screen))
  (bind _lastscreen (Variables|Default|GetLastScreen)
    (:then
      (Default|OnClose _lastscreen))
    (:else
      _))
  (Variables|Default|SetLastScreen Screen)
  (CallFunction|Initialize (Transformation|GetWorldLocation _cinecamera) _cinecamera)
  (Default|OnOpen Screen))

(event Custom|OpenLoadingScreen
  (Default|OpenLoading (Variables|/Game/ImmerseUI/Blueprints/BP_WidgetWorker.BP_WidgetWorker_C|GetMain%20UI (Variables|Default|GetWWorker))))

(event Input|EnhancedActionEvents|EnhancedInputActionIA_UIControlExit
  (params (ActionValue :type Boolean) (ElapsedSeconds :type Float%20%28double-precision%29) (TriggeredSeconds :type Float%20%28double-precision%29) (InputAction :type Input%20Action%20Object%20Reference :default "/Game/ImmerseUI/MenuInput/Actions/IA_UIControlExit.IA_UIControlExit"))
  (:Started
    (Default|CallOnExitInputPressed)))

(event Input|EnhancedActionEvents|EnhancedInputActionIA_UIControlInput1
  (params (ActionValue :type Boolean) (ElapsedSeconds :type Float%20%28double-precision%29) (TriggeredSeconds :type Float%20%28double-precision%29) (InputAction :type Input%20Action%20Object%20Reference :default "/Game/ImmerseUI/MenuInput/Actions/IA_UIControlInput1.IA_UIControlInput1"))
  (:Started
    (Default|CallOnControl1Pressed)))

(event Input|EnhancedActionEvents|EnhancedInputActionIA_UIControlInput2
  (params (ActionValue :type Boolean) (ElapsedSeconds :type Float%20%28double-precision%29) (TriggeredSeconds :type Float%20%28double-precision%29) (InputAction :type Input%20Action%20Object%20Reference :default "/Game/ImmerseUI/MenuInput/Actions/IA_UIControlInput2.IA_UIControlInput2"))
  (:Started
    (Default|CallOnControl2Pressed)))

(event EventBeginPlay
  (bind _returnvalue (Game|GetPlayerController 0))
  (bind _as玩家控制器 (Utilities|Casting|CastToPlayerController (Pawn|GetController)))
  (Utilities|IsValid (PlayerController|LocalPlayerSubsystems|GetEnhancedInputLocalPlayerSubsystem _as玩家控制器)
    (:Is%20Valid
      (Input|AddMappingContext (PlayerController|LocalPlayerSubsystems|GetEnhancedInputLocalPlayerSubsystem _as玩家控制器) "/Game/ImmerseUI/MenuInput/IMC_Menu.IMC_Menu" 0 "(bIgnoreAllPressedKeysUntilRelease=True,bForceImmediately=False,bNotifyUserSettings=False)")
      (Variables|/Script/Engine.PlayerController|SetbShowMouseCursor _returnvalue true)
      (Input|SetInputModeGameandUI _returnvalue 0 "DoNotLock" false false)
      (bind _returnvalue_2 (Actor|GetActorOfClass "/Game/ImmerseUI/Blueprints/BP_WidgetWorker.BP_WidgetWorker_C"))
      (Variables|Default|SetWWorker _returnvalue_2))))

(event Input|KeyboardEvents|DebugKeyL
  (params (Key :type Key%20Structure) (ActionValue :type Input%20Action%20Value%20Structure))
  (:Released
    (CallFunction|OpenLoadingScreen)))

(fn ConstructionScript)

(fn Initialize
  (params (NewLocation :type Vector) (Component :type Cine%20Camera%20Component%20Object%20Reference))
  (bind _cinecamera (Variables|Default|GetCineCamera))
  (Transformation|SetActorLocation NewLocation false true)
  (Variables|/Script/Engine.CameraComponent|SetPostProcessSettings _cinecamera (Variables|/Script/Engine.CameraComponent|GetPostProcessSettings Component))
  (Variables|/Script/CinematicCamera.CineCameraComponent|SetFocusSettings _cinecamera (Variables|/Script/CinematicCamera.CineCameraComponent|GetFocusSettings Component)))