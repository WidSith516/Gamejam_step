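; Worker Blueprint that creates the main UI widget, hands it a self reference and runs timeline-driven UI animations.
; It auto-slides the announcement box through three slides by lerping overlay padding and highlighting indicator dots, looping after a delay while MotionAuth is set.
; MotionAuth changes restart or stop that slideshow.
; Separate events lerp a passed widget's render translation horizontally or vertically on the chapter and character timelines.
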(event Custom|AnimateWidget
  ;[1 1 1] Announcement Box Auto Slide
  (if (Variables|/Game/ImmerseUI/Blueprints/Widgets/Components/WBPC_AnnouncementBox.WBPC_AnnouncementBox_C|GetMotionAuth (Variables|Default|GetWBPC%20Announcement%20Box))
    (Components|Timeline|SetPlayRate (Variables|Default|GetTL_SlideAnnouncementBox) (Variables|Default|GetMotionMovementRate))
    (Utilities|FlowControl|Delay (Variables|Default|GetDuration))
    (CallFunction|Move)))

(event Custom|MoveOnTimeline_SlideVertical
  (params (Transform :type Widget%20Object%20Reference%20%28by%20ref%29) (Target :type Float%20%28double-precision%29))
  (Components|Timeline|SetPlayRate (Variables|Default|GetTL_SlideCharacter) (Variables|Default|GetChapterSliderSpeed))
  (bind _float (CallFunction|StopTimileLineGetTimeCharacter))
  (bind _t1 (Timeline|TL_SlideCharacter PlayFromStart)
    (:Update
      (Variables|/Script/UMG.Widget|SetRenderTransform Transform (Utilities|Struct|MakeWidgetTransform (Math|Vector2D|MakeVector2D 0.0 (Math|Float|Lerp (.y (.translation (Variables|/Script/UMG.Widget|GetRenderTransform Transform))) Target _t1)) "(X=1.000000,Y=1.000000)" "(X=0.000000,Y=0.000000)" 0.0)))))

(event Custom|ResetAnimation
  ;[1 1 1] Announcement Box Auto Slide
  (CallFunction|ResetToggles)
  (Variables|Default|SetIndex 0)
  (CallFunction|SetToggle)
  (CallFunction|AnimateWidget))

(event Custom|MotionAuthChange
  ;[1 1 1] Initialization
  (if (Variables|/Game/ImmerseUI/Blueprints/Widgets/Components/WBPC_AnnouncementBox.WBPC_AnnouncementBox_C|GetMotionAuth (Variables|Default|GetWBPC%20Announcement%20Box))
    (CallFunction|ResetAnimation)
    (else
      (Audio|Components|Audio|Stop (Variables|Default|GetTL_SlideAnnouncementBox))
      (CallFunction|SetPadding 1.0))))

(event Custom|Move
  ;[1 1 1] Announcement Box Auto Slide
  (CallFunction|SetToggle)
  (bind _t1 (Timeline|TL_SlideAnnouncementBox PlayFromStart)
    (:Update
      (CallFunction|SetPadding _t1))
    (:Finished
      (Utilities|FlowControl|Sequence
        (:then_0
          (if (>= (+ (Variables|Default|GetIndex) 1) 3)
            (Variables|Default|SetIndex 0)
            (else
              (Variables|Default|SetIndex (+ (Variables|Default|GetIndex) 1)))))
        (:then_1
          (CallFunction|AnimateWidget))))))

(event Custom|MoveOnTilmeLine_SlideHorizontal
  (params (Transform :type Widget%20Object%20Reference%20%28by%20ref%29) (Target :type Float%20%28double-precision%29))
  (Components|Timeline|SetPlayRate (Variables|Default|GetTL_SlideChapter) (Variables|Default|GetChapterSliderSpeed))
  (bind _float (CallFunction|StopTimileLineGetTime))
  (bind _t1 (Timeline|TL_SlideChapter PlayFromStart)
    (:Update
      (Variables|/Script/UMG.Widget|SetRenderTransform Transform (Utilities|Struct|MakeWidgetTransform (Math|Vector2D|MakeVector2D (Math|Float|Lerp (.x (.translation (Variables|/Script/UMG.Widget|GetRenderTransform Transform))) Target _t1) 0.0) "(X=1.000000,Y=1.000000)" "(X=0.000000,Y=0.000000)" 0.0)))))

(event EventBeginPlay
  ;[1 1 1] Initialization
  (Utilities|FlowControl|Sequence
    (:then_0
      (bind _returnvalue (UserInterface|CreateWidget "/Game/ImmerseUI/Blueprints/Widgets/WBP_UserInterface.WBP_UserInterface_C"))
      (bind _output_get (Variables|Default|SetMain%20UI _returnvalue))
      (Variables|/Game/ImmerseUI/Blueprints/Widgets/WBP_UserInterface.WBP_UserInterface_C|SetWidgetWorker _output_get self)
      (UserInterface|Viewport|AddtoViewport _output_get 0))
    (:then_1
      (bind _output_get_2 (Variables|Default|SetWBPC%20Announcement%20Box (Variables|/Game/ImmerseUI/Blueprints/Widgets/WBP_UserInterface.WBP_UserInterface_C|GetWBPC_AnnouncementBox (Variables|Default|GetMain%20UI))))
      (Variables|/Game/ImmerseUI/Blueprints/Widgets/Components/WBPC_AnnouncementBox.WBPC_AnnouncementBox_C|SetStackSizeEspace _output_get_2 (Variables|Default|GetStackSizeEspace))
      (EventDispatchers|BindEventtoOnMotionAuthChange _output_get_2 (delegate Custom|MotionAuthChange))
      (CallFunction|ResetAnimation))))

(fn ConstructionScript)

(fn GetChildIndex
  (params (Index :type Integer) (MaxIndex :type Integer))
  (if (>= Index MaxIndex)
    (return 0)
    (else
      (return Index))))

(fn GetPrevChildIndex
  (params (Index :type Integer) (Max%20Index :type Integer))
  (bind _returnvalue (- Index 1))
  (if (< _returnvalue 0)
    (return (- Max%20Index 1))
    (else
      (return _returnvalue))))

(fn SetToggle
  (bind _wbpc_announcement_box (Variables|Default|GetWBPC%20Announcement%20Box))
  (bind _slidepoints (Variables|/Game/ImmerseUI/Blueprints/Widgets/Components/WBPC_AnnouncementBox.WBPC_AnnouncementBox_C|GetSlidePoints _wbpc_announcement_box))
  (bind _returnvalue (Class|PanelWidget|GetChildrenCount _slidepoints))
  (bind _childindex (CallFunction|GetChildIndex (Variables|Default|GetIndex) _returnvalue))
  (bind _as边界 (Utilities|Casting|CastToBorder (Class|PanelWidget|GetChildat (Variables|/Game/ImmerseUI/Blueprints/Widgets/Components/WBPC_AnnouncementBox.WBPC_AnnouncementBox_C|GetSlidePoints (Variables|Default|GetWBPC%20Announcement%20Box)) _childindex)))
  (Class|Border|SetBrushColor _as边界 "(R=1.000000,G=1.000000,B=1.000000,A=1.000000)")
  (bind _childindex_2 (CallFunction|GetPrevChildIndex _childindex _returnvalue))
  (bind _as边界_2 (Utilities|Casting|CastToBorder (Class|PanelWidget|GetChildat (Variables|/Game/ImmerseUI/Blueprints/Widgets/Components/WBPC_AnnouncementBox.WBPC_AnnouncementBox_C|GetSlidePoints (Variables|Default|GetWBPC%20Announcement%20Box)) _childindex_2)))
  (Class|Border|SetBrushColor _as边界_2 "(R=1.000000,G=1.000000,B=1.000000,A=0.000000)"))

(fn SetPadding
  (params (InputPin :type Float%20%28single-precision%29))
  (bind _wbpc_announcement_box (Variables|Default|GetWBPC%20Announcement%20Box))
  (bind _stackbox (Variables|/Game/ImmerseUI/Blueprints/Widgets/Components/WBPC_AnnouncementBox.WBPC_AnnouncementBox_C|GetStackBox _wbpc_announcement_box))
  (bind _returnvalue (Class|WidgetLayoutLibrary|SlotasOverlaySlot _stackbox))
  (Layout|BorderSlot|SetPadding _returnvalue (Utilities|Struct|MakeMargin (Math|Float|Lerp (.left (Variables|/Script/UMG.OverlaySlot|GetPadding _returnvalue)) (* (Variables|Default|GetStackSizeEspace) (Variables|Default|GetIndex)) InputPin) 0.0 0.0 0.0) :!class /Script/UMG.OverlaySlot))

(fn ResetToggles
  (for _index (range 0 (- (Class|PanelWidget|GetChildrenCount (Variables|/Game/ImmerseUI/Blueprints/Widgets/Components/WBPC_AnnouncementBox.WBPC_AnnouncementBox_C|GetSlidePoints (Variables|Default|GetWBPC%20Announcement%20Box))) 1))
    (bind _as边界 (Utilities|Casting|CastToBorder (Class|PanelWidget|GetChildat (Variables|/Game/ImmerseUI/Blueprints/Widgets/Components/WBPC_AnnouncementBox.WBPC_AnnouncementBox_C|GetSlidePoints (Variables|Default|GetWBPC%20Announcement%20Box)) _index)))
    (Class|Border|SetBrushColor _as边界 "(R=1.000000,G=1.000000,B=1.000000,A=0.000000)")))

(fn StopTimileLineGetTime
  (bind _tl_slidechapter (Variables|Default|GetTL_SlideChapter))
  (Audio|Components|Audio|Stop _tl_slidechapter)
  (return (Components|Timeline|GetPlaybackPosition _tl_slidechapter)))

(fn StopTimileLineGetTimeCharacter
  (bind _tl_slidecharacter (Variables|Default|GetTL_SlideCharacter))
  (Audio|Components|Audio|Stop _tl_slidecharacter)
  (return (Components|Timeline|GetPlaybackPosition _tl_slidecharacter)))