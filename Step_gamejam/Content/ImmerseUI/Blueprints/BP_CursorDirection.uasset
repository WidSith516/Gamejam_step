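; BP_CursorDirection tracks the mouse cursor's movement direction and fires OnDirectionChange when it turns sharply.
; A looping delay samples the DPI-scaled mouse position every 0.2 seconds, ignoring moves within an adjustable sensitivity.
; It stores the normalized previous-minus-current offset, signaling when this differs from the last by over one unit (about 60 degrees).
; GetDirection maps that offset onto the Y/Z plane, flipping the vertical axis.
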(event Custom|DetectionSettings
  (params (Sensitivity :type Float%20%28double-precision%29))
  (Variables|Default|SetDetectionSensitivity Sensitivity))

(event Custom|Step1
  (CallFunction|GetMouseLocation)
  (CallFunction|Step2))

(event Custom|Step2
  (Utilities|FlowControl|Delay 0.2)
  (CallFunction|GetLastMouseLocation)
  (CallFunction|Step1))

(event EventBeginPlay
  (CallFunction|Step1)
  (bind _returnvalue (CallFunction|GetMouseLocationVector2D))
  (Variables|Default|SetLastMotionDirection _returnvalue))

(fn GetMouseLocation
  (bind _returnvalue (Game|GetPlayerController 0))
  (bind (_locationx _locationy) (Class|WidgetLayoutLibrary|GetMousePositionScaledbyDPI _returnvalue))
  (Variables|Default|SetCapturedMouseLocation (Math|Vector2D|MakeVector2D _locationx _locationy)))

(fn GetLastMouseLocation
  (bind _returnvalue (CallFunction|GetMouseLocationVector2D))
  (if (> (Math|Float|Absolute(Float) (Math|Vector2D|Vector2DLength (- (Variables|Default|GetCapturedMouseLocation) _returnvalue))) (Variables|Default|GetDetectionSensitivity))
    (if (> (Math|Vector2D|Vector2DLength (- (Math|Vector2D|Normalize2D (- (Variables|Default|GetCapturedMouseLocation) _returnvalue)) (Variables|Default|GetLastMotionDirection))) 1.0)
      (Variables|Default|SetLastMotionDirection (Math|Vector2D|Normalize2D (- (Variables|Default|GetCapturedMouseLocation) _returnvalue)))
      (Default|CallOnDirectionChange)
      (else
        (Variables|Default|SetLastMotionDirection (Math|Vector2D|Normalize2D (- (Variables|Default|GetCapturedMouseLocation) _returnvalue)))))))

(fn GetMouseLocationVector2D
  (bind _returnvalue (Game|GetPlayerController 0))
  (bind (_locationx _locationy) (Class|WidgetLayoutLibrary|GetMousePositionScaledbyDPI _returnvalue))
  (return (Math|Vector2D|MakeVector2D _locationx _locationy)))

(fn GetDirection
  (bind _lastmotiondirection (Variables|Default|GetLastMotionDirection))
  (return (Math|Vector|MakeVector 0.0 (.x _lastmotiondirection) (* (.y _lastmotiondirection) -1.0))))